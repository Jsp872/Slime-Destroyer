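; Game mode that runs slime enemy waves and enables the mouse cursor with click and hover events.
; PopulateMap reads the current wave's data table row into a map of remaining counts per slime type.
; A looping timer spawns one enemy at a random spawn point, with ChooseEnemy re-rolling until it finds a type with stock left.
; Once none remain to spawn or alive, the timer loads the next wave.
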(event `self.ReceiveBeginPlay`
  (bind _returnvalue (`GameplayStatics.GetPlayerController` 0))
  (`|ExecutionSequence`
    (:`then_0`
      (bind _outactors (`GameplayStatics.GetAllActorsOfClass` "/Game/BP/LevelElement/SpawnAndGoal/BP_EnemiesSpawn.BP_EnemiesSpawn_C"))
      (set `self.ListOfSpawnPoint` _outactors)
      (`KismetSystemLibrary.K2_SetTimerDelegate` (delegate `ActivateSpawner`) 2.0 true)
      (`self.PopulateMap` (`self.WaveNumber`)))
    (:`then_1`
      (set `PlayerController.bShowMouseCursor` true _returnvalue)
      (set `PlayerController.bEnableClickEvents` true _returnvalue)
      (set `PlayerController.bEnableMouseOverEvents` true _returnvalue))))

(event `ActivateSpawner`
  (bind _listofspawnpoint (`self.ListOfSpawnPoint`))
  (if (> (`self.NumberOfEnemies`) 0)
    (bind _enemychosen (`self.ChooseEnemy`))
    (`/Game/BP/LevelElement/SpawnAndGoal/BP_EnemiesSpawn.SpawnEnemies` (`|GetArrayItem` _listofspawnpoint (`KismetMathLibrary.RandomIntegerInRange` 0 (- (`KismetArrayLibrary.Array_Length` _listofspawnpoint) 1))) _enemychosen)
    (else
      (bind _outactors (`GameplayStatics.GetAllActorsOfClass` "/Game/BP/Ennemies/BP_EnemyParent.BP_EnemyParent_C"))
      (if (<= (`KismetArrayLibrary.Array_Length` _outactors) 0)
        (bind _result (`/Engine/EditorBlueprintResources/StandardMacros.IncrementInt` (`self.WaveNumber`))
          (:`  `
            (`self.PopulateMap` _result)))))))

(fn `ChooseEnemy`
  (returns (EnemyChosen :type "/Game/BP/Ennemies/BP_EnemyParent Class Reference"))
  (bind _keys (`BlueprintMapLibrary.Map_Keys` (`self.EnemyList`) :!label _label))
  (bind _output_get (set `self.ChosenEnemy` (`|GetArrayItem` _keys (`KismetMathLibrary.RandomInteger` (`KismetArrayLibrary.Array_Length` _keys)))))
  (bind _value (`BlueprintMapLibrary.Map_Find` (`self.EnemyList`) _output_get))
  (set `self.EnemyNumber` _value)
  (if (> _value 0)
    (`BlueprintMapLibrary.Map_Add` (`self.EnemyList`) (`self.ChosenEnemy`) (- (`self.EnemyNumber`) 1))
    (set `self.NumberOfEnemies` (- (`self.NumberOfEnemies`) 1))
    (return (`self.ChosenEnemy`))
    (else
      (goto _label))))

(fn `PopulateMap`
  (params (WaveNumber :type Integer))
  (bind _returnvalue (`|GetDataTableRow` "/Game/BP/Ennemies/DT_WaveDetailsDataTable.DT_WaveDetailsDataTable" (`KismetStringLibrary.Conv_StringToName` (`KismetStringLibrary.Conv_IntToString` WaveNumber)))
    (:`then`
      (set `self.TotalEnemies` (+ (break `/Game/BP/Ennemies/S_WaveDetailsDataStructure` _returnvalue) (`.FastSlime_5_FAF23E544E51270219B2B6A42B5D8C0F` (break `/Game/BP/Ennemies/S_WaveDetailsDataStructure` _returnvalue)) (`.HeavySlime_6_5D4028AE468EECDA3A1FEB976E393211` (break `/Game/BP/Ennemies/S_WaveDetailsDataStructure` _returnvalue))))
      (bind _output_get (set `self.EnemyList` (`|MakeMap` "/Game/BP/Ennemies/BP_NormalSlime.BP_NormalSlime_C" (break `/Game/BP/Ennemies/S_WaveDetailsDataStructure` _returnvalue) "/Game/BP/Ennemies/BP_FastSlime.BP_FastSlime_C" (`.FastSlime_5_FAF23E544E51270219B2B6A42B5D8C0F` (break `/Game/BP/Ennemies/S_WaveDetailsDataStructure` _returnvalue)) "/Game/BP/Ennemies/BP_HeavySlime.BP_HeavySlime_C" (`.HeavySlime_6_5D4028AE468EECDA3A1FEB976E393211` (break `/Game/BP/Ennemies/S_WaveDetailsDataStructure` _returnvalue)) :!type "/Game/BP/Ennemies/BP_EnemyParent Class Reference")))
      (bind _values (`BlueprintMapLibrary.Map_Values` _output_get))
      (for _array_element _values
        (set `self.NumberOfEnemies` (+ _array_element (`self.NumberOfEnemies`)))))))

(fn `UserConstructionScript`)