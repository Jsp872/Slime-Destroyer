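; BP_Archer is an adventurer level element that automatically and repeatedly fires arrow projectiles.
; Tick drives a short Delay into Shot, which spawns a BP_ProjectileArrow at the ShootZone transform and stores it in Bullet.
; A longer Delay then destroys whatever Bullet references; since each shot overwrites it and shots outpace that Delay, only the latest arrow is destroyed.
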(event `self.ReceiveTick`
  (params (DeltaSeconds :type "Float (single-precision)"))
  (`KismetSystemLibrary.Delay` 0.25)
  (`self.Shot` self)
  (`KismetSystemLibrary.Delay` 5.0)
  (`self.K2_DestroyActor` (`self.Bullet`)))

(fn `Shot`
  (bind _returnvalue (`|SpawnActorFromClass` "/Game/BP/LevelElement/Adventurers/BP_ProjectileArrow.BP_ProjectileArrow_C" (`SceneComponent.K2_GetComponentToWorld` (`self.ShootZone`)) "Undefined" "MultiplyWithRoot" null null))
  (set `self.Bullet` _returnvalue))

(fn `UserConstructionScript`)