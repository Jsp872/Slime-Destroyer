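; Base projectile actor for adventurers, which damages enemies derived from BP_EnemyParent when its box collision hits them.
; On BeginPlay it copies its gravity, initial speed and max speed variables into ProjectileMovement and sets its lifespan.
; Any box hit, enemy or not, spawns the slime impact Niagara effect, plays a 2D hit sound and destroys the projectile.
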(event `self.ReceiveBeginPlay`
  (bind _projectilemovement (`self.ProjectileMovement`))
  (set `ProjectileMovementComponent.ProjectileGravityScale` (`self.ProjectileGravity`) _projectilemovement)
  (set `ProjectileMovementComponent.InitialSpeed` (`self.ProjectileInitialSpeed`) _projectilemovement)
  (set `ProjectileMovementComponent.MaxSpeed` (`self.ProjectileMaxSpeed`) _projectilemovement)
  (`self.SetLifeSpan` self (`self.ProjectileLifeTime`)))

(event `self.Box.OnComponentHit`
  (params (HitComponent :type "PrimitiveComponent Object Reference") (OtherActor :type "Actor Object Reference") (OtherComp :type "PrimitiveComponent Object Reference") (NormalImpulse :type "Vector Structure") (Hit :type "HitResult Structure (by ref)"))
  (`|ExecutionSequence`
    (:`then_0`
      (bind _asbp_enemy_parent (cast `/Game/BP/Ennemies/BP_EnemyParent` OtherActor))
      (`GameplayStatics.ApplyDamage` _asbp_enemy_parent (`self.DamageProjectile`)))
    (:`then_1`
      (`NiagaraFunctionLibrary.SpawnSystemAtLocation` "/Game/BP/LevelElement/Adventurers/Projectile/NS_HitSlime.NS_HitSlime" (`self.K2_GetActorLocation`))
      (`GameplayStatics.SpawnSound2D` "/Game/Sound/Sfx/SC_SlimeHit.SC_SlimeHit" 1.0 1.0 0.0 null)
      (`self.K2_DestroyActor`))))

(fn `UserConstructionScript`)