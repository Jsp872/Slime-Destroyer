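; BP_PurseSlot is a clickable purse marking a placement slot where adventurers, acting as turrets, are selected or upgraded.
; Cursor events swap the purse material for hover, pressed and idle feedback.
; A click hides open menus, then shows the select widget if CanSpawnATurret is true, otherwise the upgrade widget for the current adventurer.
; Both widgets are created lazily, cached on the HUD and retargeted to the clicked slot on reuse.
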(event `self.ReceiveBeginPlay`
  (bind _ashud_hud (cast `/Game/BP/HUD/HUD_HUD` (`PlayerController.GetHUD` (`GameplayStatics.GetPlayerController` 0))))
  (set `self.As HUD HUD` _ashud_hud))

(event `self.Purse.OnBeginCursorOver`
  (params (TouchedComponent :type "PrimitiveComponent Object Reference"))
  (`PrimitiveComponent.SetMaterial` (`self.Purse`) 0 "/Game/Material/M_PurseMouseOver.M_PurseMouseOver"))

(event `self.Purse.OnEndCursorOver`
  (params (TouchedComponent :type "PrimitiveComponent Object Reference"))
  (`PrimitiveComponent.SetMaterial` (`self.Purse`) 0 "/Game/Material/M_PurseMouseOut.M_PurseMouseOut"))

(event `self.Purse.OnClicked`
  (params (TouchedComponent :type "PrimitiveComponent Object Reference") (ButtonPressed :type "Key Structure"))
  (bind _currentselectwidget (`/Game/BP/HUD/HUD_HUD.CurrentSelectWidget` (`self.As HUD HUD`)))
  (bind _currentselectwidget_2 (`/Game/BP/HUD/HUD_HUD.CurrentSelectWidget` (`self.As HUD HUD`)))
  (bind _currentupgradewidget (`/Game/BP/HUD/HUD_HUD.CurrentUpgradeWidget` (`self.As HUD HUD`)))
  (`PrimitiveComponent.SetMaterial` (`self.Purse`) 0 "/Game/Material/M_PurseMouseClicked.M_PurseMouseClicked")
  (`/Engine/EditorBlueprintResources/StandardMacros.IsValid` _currentselectwidget_2
    (:`Is Valid`
      (`Widget.SetVisibility` _currentselectwidget_2 "Hidden"))
    (:`Is Not Valid`
      _))
  (`/Engine/EditorBlueprintResources/StandardMacros.IsValid` _currentupgradewidget
    (:`Is Valid`
      (`Widget.SetVisibility` _currentupgradewidget "Hidden"))
    (:`Is Not Valid`
      _))
  (if (`self.CanSpawnATurret`)
    (if (== _currentselectwidget null)
      (bind _returnvalue (`|CreateWidget` "/Game/BP/HUD/WBP_AdventurerSelect.WBP_AdventurerSelect_C" null null))
      (`UserWidget.AddToViewport` _returnvalue 0)
      (set `/Game/BP/HUD/WBP_AdventurerSelect.EmptySlot` self _returnvalue)
      (set `/Game/BP/HUD/HUD_HUD.CurrentSelectWidget` _returnvalue (`self.As HUD HUD`))
      (else
        (set `/Game/BP/HUD/WBP_AdventurerSelect.EmptySlot` self _currentselectwidget)
        (`Widget.SetVisibility` _currentselectwidget "SelfHitTestInvisible")))
    (elif (== _currentupgradewidget null)
      (bind _returnvalue_2 (`|CreateWidget` "/Game/BP/HUD/WBP_AdventurerUpgrade.WBP_AdventurerUpgrade_C" null null))
      (`UserWidget.AddToViewport` _returnvalue_2 0)
      (set `/Game/BP/HUD/WBP_AdventurerUpgrade.EmptySlot` self _returnvalue_2)
      (set `/Game/BP/HUD/WBP_AdventurerUpgrade.SelectedAdventurer` (`self.CurrentAdventurer`) _returnvalue_2)
      (set `/Game/BP/HUD/HUD_HUD.CurrentUpgradeWidget` _returnvalue_2 (`self.As HUD HUD`))
      (`/Game/BP/HUD/WBP_AdventurerUpgrade.Refresh` (`/Game/BP/HUD/HUD_HUD.CurrentUpgradeWidget` (`self.As HUD HUD`)))
      (else
        (set `/Game/BP/HUD/WBP_AdventurerUpgrade.SelectedAdventurer` (`self.CurrentAdventurer`) _currentupgradewidget)
        (set `/Game/BP/HUD/WBP_AdventurerUpgrade.EmptySlot` self _currentupgradewidget)
        (`/Game/BP/HUD/WBP_AdventurerUpgrade.Refresh` _currentupgradewidget)
        (`Widget.SetVisibility` _currentupgradewidget "SelfHitTestInvisible")
        (`/Game/BP/HUD/WBP_AdventurerUpgrade.Refresh` (`/Game/BP/HUD/HUD_HUD.CurrentUpgradeWidget` (`self.As HUD HUD`)))))))

(event `self.Purse.OnReleased`
  (params (TouchedComponent :type "PrimitiveComponent Object Reference") (ButtonReleased :type "Key Structure"))
  (`PrimitiveComponent.SetMaterial` (`self.Purse`) 0 "/Game/Material/M_PurseMouseOver.M_PurseMouseOver"))

(fn `UserConstructionScript`)