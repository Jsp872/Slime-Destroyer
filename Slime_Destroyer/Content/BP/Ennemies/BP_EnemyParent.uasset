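; BP_EnemyParent is the base tower defense enemy, which walks to the BP_GoalOfEnemies actor using AIMoveTo, retrying on failure.
; Reaching the goal destroys it, decrements the GM_Game enemy count and takes player life through PC_TowerDefense, showing a paused game-over screen at zero life.
; Damage reduces Hp; at zero it is destroyed and awards resources to the player, without decrementing the enemy count here.
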(event `self.ReceiveBeginPlay`
  (`self.GoToGoal`))

(event `GoToGoal`
  (if (`self.HpGood?`)
    (`KismetSystemLibrary.Delay` 0.2)
    (set `CharacterMovementComponent.MaxWalkSpeed` (`self.MoveSpeed`) (`self.CharacterMovement`))
    (bind _outactors (`GameplayStatics.GetAllActorsOfClass` "/Game/BP/LevelElement/SpawnAndGoal/BP_GoalOfEnemies.BP_GoalOfEnemies_C"))
    (`|AIMoveTo` self (0.0 0.0 0.0) (`|GetArrayItem` _outactors) 200.0
      (:`OnSuccess`
        (`self.K2_DestroyActor`)
        (bind _asgm_game (cast `/Game/BP/GM_Game` (`GameplayStatics.GetGameMode`)))
        (bind _output_get (set `self.GameMode` _asgm_game))
        (set `/Game/BP/GM_Game.TotalEnemies` (- (`/Game/BP/GM_Game.TotalEnemies` _output_get) 1) _output_get)
        (bind _aspc_tower_defense (cast `/Game/BP/PC_TowerDefense` (`GameplayStatics.GetPlayerController` 0)))
        (`/Game/BP/PC_TowerDefense.Take Life` _aspc_tower_defense (`self.LifeTaken`))
        (if (<= (`/Game/BP/PC_TowerDefense.Life` _aspc_tower_defense) 0)
          (set `/Game/BP/PC_TowerDefense.Life` 0 _aspc_tower_defense)
          (bind _returnvalue (`|CreateWidget` "/Game/BP/HUD/WBP_GameOver.WBP_GameOver_C"))
          (`UserWidget.AddToViewport` _returnvalue 0)
          (`GameplayStatics.SetGamePaused` true)))
      (:`OnFail`
        (`self.GoToGoal`)))))

(event `self.ReceiveAnyDamage`
  (params (Damage :type "Float (single-precision)") (DamageType :type "DamageType Object Reference") (InstigatedBy :type "Controller Object Reference") (DamageCauser :type "Actor Object Reference"))
  (bind _hp (`self.Hp`))
  (set `self.Hp` (- _hp Damage))
  (if (<= _hp 0.0)
    (`SceneComponent.SetVisibility` (`self.WidgetHpEnemy`) false false)
    (set `CharacterMovementComponent.MaxWalkSpeed` 0.0 (`self.CharacterMovement`))
    (set `self.HpGood?` false)
    (`PrimitiveComponent.SetCollisionEnabled` (`self.CapsuleComponent`) "NoCollision")
    (`self.K2_DestroyActor`)
    (bind _aspc_tower_defense (cast `/Game/BP/PC_TowerDefense` (`GameplayStatics.GetPlayerController` 0)))
    (`/Game/BP/PC_TowerDefense.AddResources` _aspc_tower_defense (`self.ResourceGiveWhenDead`))))

(fn `UserConstructionScript`)